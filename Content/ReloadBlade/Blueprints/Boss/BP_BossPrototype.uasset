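; Prototype boss that fights the top-down player character with a telegraphed, range-checked melee attack on a cooldown.
; Gun Q and W hits add Cutting or Impact marks, which Sword skills consume for bonus health damage or, for Impact marks, posture damage.
; Depleted posture staggers the boss, blocking attacks until it recovers, while zero health hides the mesh and disables its collision.
; Feedback is debug-only, using printed strings and a warning sphere.
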(event Custom|StartBossStagger
  ;[0.15 0.15 0.15 0.5] Boss Staggered
  (Variables|Default|SetIsStaggered true)
  (Development|PrintString "BOSS STAGGERED")
  (Utilities|FlowControl|Delay 4.0)
  (Variables|Default|SetCurrentPosture (Variables|Default|GetMaxPosture))
  (Variables|Default|SetIsStaggered false)
  (Development|PrintString "BOSS RECOVERED"))

(event Custom|StartMeleeCooldown
  ;[0.15 0.15 0.15 0.5] Boss Melee Attack
  ;;[0.15 0.15 0.15 0.5] StartMeleeCooldown
  (Utilities|FlowControl|Delay 2.0)
  (Variables|Default|SetCanMeleeAttack true))

(event EventBeginPlay)

(event Collision|EventActorBeginOverlap
  (params (OtherActor :type Actor%20Object%20Reference)))

(event EventTick
  (params (DeltaSeconds :type Float%20%28single-precision%29))
  ;[0.15 0.15 0.15 0.5] Boss Melee Attack
  (bind _asbp_top_down_character (Utilities|Casting|CastToBP_TopDownCharacter (Game|GetPlayerCharacter 0)))
  (if (Math|Boolean|ANDBoolean (not (Variables|/Game/TopDown/Blueprints/BP_TopDownCharacter.BP_TopDownCharacter_C|GetIsDead _asbp_top_down_character)) (<= (Math|Vector|Distance(Vector) (Transformation|GetActorLocation) (Transformation|GetActorLocation _asbp_top_down_character)) (Variables|Default|GetMeleeAttackRange)) (Variables|Default|GetCanMeleeAttack) (not (Variables|Default|GetIsDead)) (not (Variables|Default|GetIsStaggered)))
    (Variables|Default|SetCanMeleeAttack false)
    (Development|PrintString "BOSS MELEE WARNING(0.8s)")
    (Rendering|Debug|DrawDebugSphere (Transformation|GetActorLocation) (Variables|Default|GetMeleeAttackRange) 32 "(R=0.252174,G=0.000000,B=0.004786,A=1.000000)" 0.8 4.0)
    (Utilities|FlowControl|Delay 0.8)
    (if (Math|Boolean|ANDBoolean (<= (Math|Vector|Distance(Vector) (Transformation|GetActorLocation) (Transformation|GetActorLocation _asbp_top_down_character)) (Variables|Default|GetMeleeAttackRange)) (not (Variables|/Game/TopDown/Blueprints/BP_TopDownCharacter.BP_TopDownCharacter_C|GetIsDead _asbp_top_down_character)) (not (Variables|Default|GetIsDead)) (not (Variables|Default|GetIsStaggered)))
      (Development|PrintString "BOSS MELEE ATTACK")
      (Default|ReceivePlayerDamage _asbp_top_down_character 2e+01)
      (CallFunction|StartMeleeCooldown)
      (else
        (CallFunction|StartMeleeCooldown)))))

(fn ConstructionScript)

(fn ReceiveGunQDamage
  (if (not (Variables|Default|GetIsDead))
    (bind _output_get (Variables|Default|SetCurrentHealth (Math|Float|Clamp(Float) (- (Variables|Default|GetCurrentHealth) 3e+01) 0.0 (Variables|Default|GetMaxHealth))))
    (Development|PrintString (Utilities|String|ToString(Float) _output_get))
    (bind _output_get_2 (Variables|Default|SetCuttingMarkCount (Math|Integer|Clamp(Integer) (+ (Variables|Default|GetCuttingMarkCount) 1) 0 4)))
    (Development|PrintString (Utilities|String|ToString(Integer) _output_get_2))
    (CallFunction|CheckBossDeath)))

(fn ReceiveSwordQDamage
  (if (not (Variables|Default|GetIsDead))
    (if (> (Variables|Default|GetCuttingMarkCount) 0)
      (bind _output_get (Variables|Default|SetCurrentHealth (Math|Float|Clamp(Float) (- (Variables|Default|GetCurrentHealth) 1.6e+02) 0.0 (Variables|Default|GetMaxHealth))))
      (bind _output_get_2 (Variables|Default|SetCuttingMarkCount (- (Variables|Default|GetCuttingMarkCount) 1)))
      (Development|PrintString (Utilities|String|ToString(Integer) _output_get_2))
      (Development|PrintString (Utilities|String|ToString(Float) _output_get))
      (CallFunction|CheckBossDeath)
      (else
        (bind _output_get_3 (Variables|Default|SetCurrentHealth (Math|Float|Clamp(Float) (- (Variables|Default|GetCurrentHealth) 6e+01) 0.0 (Variables|Default|GetMaxHealth))))
        (Development|PrintString (Utilities|String|ToString(Float) _output_get_3))
        (CallFunction|CheckBossDeath)))))

(fn ReceiveGunWDamage
  (if (not (Variables|Default|GetIsDead))
    (bind _output_get (Variables|Default|SetCurrentHealth (Math|Float|Clamp(Float) (- (Variables|Default|GetCurrentHealth) 2e+01) 0.0 (Variables|Default|GetMaxHealth))))
    (Development|PrintString (Utilities|String|ToString(Float) _output_get))
    (bind _output_get_2 (Variables|Default|SetImpactMarkCount (Math|Integer|Clamp(Integer) (+ (Variables|Default|GetImpactMarkCount) 1) 0 4)))
    (Development|PrintString (Utilities|String|ToString(Integer) _output_get_2))
    (CallFunction|CheckBossDeath)))

(fn ReceiveSwordWDamage
  (if (not (Variables|Default|GetIsDead))
    (bind _output_get (LocalVariables|SetCuttingMarksToConsume (Math|Integer|Min(Integer) (Variables|Default|GetCuttingMarkCount) 3)))
    (LocalVariables|SetRemainingConsumeSlots (- 3 (LocalVariables|GetCuttingMarksToConsume)))
    (bind _output_get_2 (LocalVariables|SetImpactMarksToConsume (Math|Integer|Min(Integer) (Variables|Default|GetImpactMarkCount) (LocalVariables|GetRemainingConsumeSlots))))
    (bind _output_get_3 (LocalVariables|SetTotalDamage (Math|Conversions|ToFloat(Integer) (+ (* (LocalVariables|GetCuttingMarksToConsume) 80) 100))))
    (bind _output_get_4 (LocalVariables|SetTotalPostureDamage (Math|Conversions|ToFloat(Integer) (* (LocalVariables|GetImpactMarksToConsume) 80))))
    (bind _output_get_5 (Variables|Default|SetCurrentHealth (Math|Float|Clamp(Float) (- (Variables|Default|GetCurrentHealth) _output_get_3) 0.0 (Variables|Default|GetMaxHealth))))
    (bind _output_get_6 (Variables|Default|SetCuttingMarkCount (- (Variables|Default|GetCuttingMarkCount) _output_get)))
    (bind _output_get_7 (Variables|Default|SetImpactMarkCount (- (Variables|Default|GetImpactMarkCount) _output_get_2)))
    (CallFunction|ApplyPostureDamage _output_get_4)
    (Development|PrintString (Utilities|String|ToString(Float) _output_get_3))
    (Development|PrintString (Utilities|String|ToString(Float) _output_get_5))
    (Development|PrintString (Utilities|String|ToString(Integer) _output_get_6))
    (Development|PrintString (Utilities|String|ToString(Integer) _output_get_7))
    (CallFunction|CheckBossDeath)))

(fn CheckBossDeath
  (bind _bossmesh (Variables|Default|GetBossMesh))
  (if (<= (Variables|Default|GetCurrentHealth) 0.0)
    (Variables|Default|SetIsDead true)
    (Development|PrintString "BOSS DEAD")
    (Collision|SetCollisionEnabled _bossmesh "NoCollision")
    (Rendering|SetVisibility _bossmesh false true)))

(fn ApplyPostureDamage
  (params (DamageAmount :type Float%20%28double-precision%29))
  (if (and (not (Variables|Default|GetIsDead)) (not (Variables|Default|GetIsStaggered)))
    (bind _output_get (Variables|Default|SetCurrentPosture (Math|Float|Clamp(Float) (- (Variables|Default|GetCurrentPosture) DamageAmount) 0.0 (Variables|Default|GetMaxPosture))))
    (Development|PrintString (Utilities|String|ToString(Float) _output_get))
    (CallFunction|CheckBossStagger)))

(fn CheckBossStagger
  (if (and (<= (Variables|Default|GetCurrentPosture) 0.0) (not (Variables|Default|GetIsStaggered)))
    (CallFunction|StartBossStagger)))